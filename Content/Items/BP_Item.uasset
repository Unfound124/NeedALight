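; BP_Item is an item actor that responds to cursor hover to mark itself as a pickup candidate for the player.
; On BeginPlay it copies the item name into its pickup widget and caches the player pawn.
; Hovering the collision always shows the glow, but shows the widget and sets the player's CurrentHover only within PickupDistance.
; Ending the hover hides both and clears CurrentHover.
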(event OnBeginCursorOver(Collision)
  (params (TouchedComponent :type Primitive%20Component%20Object%20Reference))
  (if (<= (Transformation|GetDistanceTo (Game|Player|GetPlayerPawn 0)) (Variables|Default|GetPickupDistance))
    (Rendering|SetVisibility (Variables|Default|GetPickupWidget) true false)
    (Variables|/Game/Player/Player.Player_C|SetCurrentHover (Variables|Default|GetPlayerRef) self))
  (Rendering|SetVisibility (Variables|Default|GetGlow) true false))

(event OnEndCursorOver(Collision)
  (params (TouchedComponent :type Primitive%20Component%20Object%20Reference))
  (Rendering|SetVisibility (Variables|Default|GetGlow) false false)
  (Variables|/Game/Player/Player.Player_C|SetCurrentHover (Variables|Default|GetPlayerRef) 0))

(event EventBeginPlay
  (bind _aspick_up_object (Utilities|Casting|CastToPickUpObject (UserInterface|GetUserWidgetObject (Variables|Default|GetPickupWidget))))
  (Variables|/Game/Widgets/PickUpObject.PickUpObject_C|SetitemName _aspick_up_object (.Name (Utilities|Struct|BreakItemInfo (Variables|Default|GetitemInfo))))
  (bind _asplayer (Utilities|Casting|CastToPlayer (Game|Player|GetPlayerPawn 0)))
  (Variables|Default|SetPlayerRef _asplayer))

(event Collision|EventActorBeginOverlap
  (params (OtherActor :type Actor%20Object%20Reference)))

(event EventTick
  (params (DeltaSeconds :type Float%20%28single-precision%29)))

(fn ConstructionScript)